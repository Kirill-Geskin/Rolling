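; Explosive pickup, a child of a pickup base Blueprint, that blasts the ball pawn on pickup.
; BeginPlay disables the widget flag, sets an explosion sound and emitter for the parent's pickup logic, and plays a sparks sound at its location.
; OnPickup casts to BallPawn and applies a mass-independent radial impulse from just below the pickup to the ball mesh, then calls the parent handler.
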(event EventBeginPlay
  (Variables|Default|SetUseWidgetBool false) ; Var. UseWidgetBool == false
  (Variables|Default|SetOnPickupSound "/Game/StarterContent/Audio/Explosion01.Explosion01") ; SET for pickup sound
  (Variables|Default|SetEmitterTemplateForPickup "/Game/StarterContent/Particles/P_Explosion.P_Explosion") ; SET for pickup Emitter
  (Audio|PlaySoundatLocation "/Game/Blueprints/Pickup/Sounds/Fire_Sparks01_Cue.Fire_Sparks01_Cue" (Transformation|GetActorLocation) "0.000000, 0, 0" 1.0 1.0 0.0 0 0 0)
  (|CallParentFunction))

(event Collision|EventActorBeginOverlap
  (params (OtherActor :type Actor%20Object%20Reference))
  (|CallParentFunction OtherActor) ; This node is disabled and will not be called.\nDrag off pins to build functionality.
)

(event EventTick
  (params (DeltaSeconds :type Float%20%28single-precision%29))
  (|CallParentFunction DeltaSeconds) ; This node is disabled and will not be called.\nDrag off pins to build functionality.
)

(event EventOnPickup
  (params (Object :type Object%20Object%20Reference))
  (bind _returnvalue (Transformation|GetActorLocation))
  (bind (_x _y _z) (Math|Vector|BreakVector _returnvalue))
  (bind _asball_pawn (Utilities|Casting|CastToBallPawn Object))
  (Physics|AddRadialImpulse (Variables|/Game/Blueprints/BallPawn.BallPawn_C|GetBallMesh _asball_pawn) (Math|Vector|MakeVector _x _y (- _z 5e+01)) 5e+02 7.5e+02 "RIF_Constant" true)
  (|CallParentFunction Object))

(fn ConstructionScript
  (|CallParentFunction))